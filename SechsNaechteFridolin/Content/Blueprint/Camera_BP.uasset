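; Camera_BP is a possessable camera with an attached spotlight that lights up only while it is possessed.
; The light starts hidden at BeginPlay, is shown on possession and is hidden again on unpossession.
; A BigRoom flag makes BeginPlay boost the spotlight's intensity and attenuation radius for larger spaces.
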(event `self.ReceivePossessed`
  (params (NewController :type "Controller Object Reference"))
  (`SceneComponent.SetHiddenInGame` (`self.SpotLight`) false false))

(event `self.ReceiveUnpossessed`
  (params (OldController :type "Controller Object Reference"))
  (`SceneComponent.SetHiddenInGame` (`self.SpotLight`) true false))

(event `self.ReceiveBeginPlay`
  (bind _spotlight (`self.SpotLight`))
  (bind _spotlight_2 (`self.SpotLight`))
  (`SceneComponent.SetHiddenInGame` (`self.SpotLight`) true false)
  (if (`self.BigRoom`)
    (`LightComponent.SetIntensity` _spotlight (* (`LightComponentBase.Intensity` _spotlight) 3.0))
    (`LocalLightComponent.SetAttenuationRadius` _spotlight_2 (* (`LocalLightComponent.AttenuationRadius` _spotlight_2) 2.0))))

(fn `UserConstructionScript`)