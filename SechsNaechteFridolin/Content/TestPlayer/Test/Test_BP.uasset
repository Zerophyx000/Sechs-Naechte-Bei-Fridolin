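; Test first-person player character with movement, mouse-look, a toggleable flashlight and an interact action.
; Interact runs a short visibility line trace from the camera, ignoring itself, prints the hit actor's name and sends it InteractMessage with the player as argument.
; A FlipFlop alternately hides and shows the flashlight, hiding it on the first press.
; Unconnected leftover nodes for possession and resetting HackedPCS never run.
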(event `InputAction|Interact`
  (params (Key :type "Key Structure"))
  (bind _camera (`self.Camera`))
  (bind _returnvalue (`SceneComponent.K2_GetComponentLocation` _camera))
  (:`Pressed`
    (bind _outhit (`KismetSystemLibrary.LineTraceSingle` _returnvalue (+ _returnvalue (* (`KismetMathLibrary.GetForwardVector` (`SceneComponent.K2_GetComponentRotation` _camera)) 300.0)) "TraceTypeQuery1" false (`self.IgnoredActors`)))
    (`KismetSystemLibrary.PrintString` (`KismetSystemLibrary.GetDisplayName` (`.HitActor` (`GameplayStatics.BreakHitResult` _outhit))))
    (message `/Game/TestPlayer/Test/Interaction.Interact` (`.HitActor` (`GameplayStatics.BreakHitResult` _outhit)) self)))

(event `self.ReceiveBeginPlay`
  (`KismetArrayLibrary.Array_Add` (`self.IgnoredActors`) self))

(event `InputAction|Toggle Flashlight`
  (params (Key :type "Key Structure"))
  (:`Pressed`
    (`/Engine/EditorBlueprintResources/StandardMacros.FlipFlop`
      (:`A`
        (`SceneComponent.SetHiddenInGame` (`self.Flashlight`) true false))
      (:`B`
        (`SceneComponent.SetHiddenInGame` (`self.Flashlight`) false false)))))

(event `InputAxis|LookRight`
  (params (AxisValue :type "Float (single-precision)"))
  (`self.AddControllerYawInput` AxisValue))

(event `InputAxis|GoUp`
  (params (AxisValue :type "Float (single-precision)"))
  (`self.AddMovementInput` (`SceneComponent.GetForwardVector` (`self.CapsuleComponent`)) AxisValue))

(event `InputAxis|LookUp`
  (params (AxisValue :type "Float (single-precision)"))
  (`self.AddControllerPitchInput` AxisValue))

(event `InputAxis|GoRight`
  (params (AxisValue :type "Float (single-precision)"))
  (`self.AddMovementInput` (`SceneComponent.GetRightVector` (`self.CapsuleComponent`)) AxisValue))

(fn `UserConstructionScript`)