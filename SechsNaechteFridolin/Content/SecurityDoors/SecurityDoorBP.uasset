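; Security door actor that alternates between rising and lowering each time ToggleDoor is called.
; A FlipFlop plays one of two timelines, each nudging Z via FInterpTo toward an offset from the current height, so travel depends on timeline length.
; Particle and Niagara effects switch on or off at each movement's start and end.
; The linked Button receives DoorClosing false at the start and true on finish.
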(event `self.ReceiveTick`
  (params (DeltaSeconds :type "Float (single-precision)")))

(event `Toggle Door`
  (bind (_returnvalue_x _returnvalue_y _returnvalue_z) (`KismetMathLibrary.BreakVector` (`self.K2_GetActorLocation`)))
  (bind (_returnvalue_x_2 _returnvalue_y_2 _returnvalue_z_2) (`KismetMathLibrary.BreakVector` (`self.K2_GetActorLocation`)))
  (bind (_returnvalue_x_3 _returnvalue_y_3 _returnvalue_z_3) (`KismetMathLibrary.BreakVector` (`self.K2_GetActorLocation`)))
  (bind _niagara (`self.Niagara`))
  (bind _button (`self.Button`))
  (bind _button_2 (`self.Button`))
  (set `self.DoorHeight` _returnvalue_z_3)
  (`/Engine/EditorBlueprintResources/StandardMacros.FlipFlop`
    (:`A`
      (`/Game/SecurityDoors/DoorButtonBP.DoorClosing` _button_2 false)
      (`ActorComponent.Activate` (`self.ParticleSystem`) true)
      (`ActorComponent.Activate` (`self.ParticleSystem1`) true)
      (`ActorComponent.Activate` _niagara false)
      (`Timeline|Timeline` :!via `PlayFromStart`
        (:`Update`
          (`self.K2_SetActorLocation` (`KismetMathLibrary.MakeVector` _returnvalue_x_2 _returnvalue_y_2 (`KismetMathLibrary.FInterpTo` _returnvalue_z_2 (+ _returnvalue_z_2 75.0) (stale `self.ReceiveTick` DeltaSeconds) 1.0))))
        (:`Finished`
          (`/Game/SecurityDoors/DoorButtonBP.DoorClosing` _button true)
          (`ActorComponent.Deactivate` (`self.Niagara1`))
          (`ActorComponent.Deactivate` (`self.Niagara2`)))))
    (:`B`
      (`/Game/SecurityDoors/DoorButtonBP.DoorClosing` _button_2 false)
      (`ActorComponent.Deactivate` (`self.ParticleSystem`))
      (`ActorComponent.Deactivate` (`self.ParticleSystem1`))
      (`ActorComponent.Deactivate` _niagara)
      (`Timeline|Timeline_0` :!via `PlayFromStart`
        (:`Update`
          (`self.K2_SetActorLocation` (`KismetMathLibrary.MakeVector` _returnvalue_x _returnvalue_y (`KismetMathLibrary.FInterpTo` _returnvalue_z (- _returnvalue_z 75.0) (stale `self.ReceiveTick` DeltaSeconds) 1.0))))
        (:`Finished`
          (`/Game/SecurityDoors/DoorButtonBP.DoorClosing` _button true)
          (`ActorComponent.Activate` (`self.Niagara2`) false)
          (`ActorComponent.Activate` (`self.Niagara1`) false))))))

(fn `UserConstructionScript`)